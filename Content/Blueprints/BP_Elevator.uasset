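; BP_Elevator is an elevator actor whose platform moves between Start and End transforms when something overlaps its bottom or top entry trigger.
; Each trigger waits briefly, then plays its own timeline from the start, whose track drives a transform lerp setting the platform's location and rotation.
; Timeline event tracks swap the platform material between active while moving and ready when stopped.
; Overlaps are not filtered by actor.
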(event OnComponentBeginOverlap(BottomEntry)
  (params (OverlappedComponent :type Primitive%20Component%20Object%20Reference) (OtherActor :type Actor%20Object%20Reference) (OtherComp :type Primitive%20Component%20Object%20Reference) (OtherBodyIndex :type Integer) (bFromSweep :type Boolean) (SweepResult :type Hit%20Result%20Structure%20%28by%20ref%29))
  (Utilities|FlowControl|Delay 1.0)
  (bind _newtrack_1 (Timeline|Timeline_0 PlayFromStart)
    (:Update
      (Transformation|SetWorldLocationAndRotation (Variables|Default|GetPlatform) (.location (Math|Transform|Lerp(Transform) (Transformation|GetWorldTransform (Variables|Default|GetStart)) (Transformation|GetWorldTransform (Variables|Default|GetEnd)) _newtrack_1)) (.rotation (Math|Transform|Lerp(Transform) (Transformation|GetWorldTransform (Variables|Default|GetStart)) (Transformation|GetWorldTransform (Variables|Default|GetEnd)) _newtrack_1)) false false))
    (:Moving
      (Rendering|Material|SetMaterial (Variables|Default|GetPlatform) 0 "/Game/Materials/FallingPlatforms/MI_ActivePlatform.MI_ActivePlatform"))
    (:Stopped
      (Rendering|Material|SetMaterial (Variables|Default|GetPlatform) 0 "/Game/Materials/FallingPlatforms/MI_ReadyPlatform.MI_ReadyPlatform"))))

(event OnComponentBeginOverlap(TopEntry)
  (params (OverlappedComponent :type Primitive%20Component%20Object%20Reference) (OtherActor :type Actor%20Object%20Reference) (OtherComp :type Primitive%20Component%20Object%20Reference) (OtherBodyIndex :type Integer) (bFromSweep :type Boolean) (SweepResult :type Hit%20Result%20Structure%20%28by%20ref%29))
  (Utilities|FlowControl|Delay 1.0)
  (bind _newtrack_0 (Timeline|Timeline_1 PlayFromStart)
    (:Update
      (Transformation|SetWorldLocationAndRotation (Variables|Default|GetPlatform) (.location (Math|Transform|Lerp(Transform) (Transformation|GetWorldTransform (Variables|Default|GetStart)) (Transformation|GetWorldTransform (Variables|Default|GetEnd)) _newtrack_0)) (.rotation (Math|Transform|Lerp(Transform) (Transformation|GetWorldTransform (Variables|Default|GetStart)) (Transformation|GetWorldTransform (Variables|Default|GetEnd)) _newtrack_0)) false false))
    (:Moving
      (Rendering|Material|SetMaterial (Variables|Default|GetPlatform) 0 "/Game/Materials/FallingPlatforms/MI_ActivePlatform.MI_ActivePlatform"))
    (:Stopped
      (Rendering|Material|SetMaterial (Variables|Default|GetPlatform) 0 "/Game/Materials/FallingPlatforms/MI_ReadyPlatform.MI_ReadyPlatform"))))

(event EventBeginPlay)

(event Collision|EventActorBeginOverlap
  (params (OtherActor :type Actor%20Object%20Reference)))

(event EventTick
  (params (DeltaSeconds :type Float%20%28single-precision%29)))

(fn ConstructionScript)